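; BP_HW_Actor is a test actor that exercises a line trace and a health counter through on-screen debug prints.
; BeginPlay starts two looping timers: the fast one prints Health and draws a visibility trace from the actor to LineTraceFunction's endpoint, ignoring the hit.
; The slower one increments Health and prints LimitHealthFunction's result.
; LaneTraceFunctionBP computes a forward endpoint from MaxDistance but is not called here.
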(event `self.ReceiveBeginPlay`
  (`KismetSystemLibrary.K2_SetTimerDelegate` (delegate `TimerTest`) 0.01 true true)
  (`KismetSystemLibrary.K2_SetTimerDelegate` (delegate `mainTime`) 0.1 true true))

(event `TimerTest`
  (`|ExecutionSequence`
    (:`then_0`
      (`KismetSystemLibrary.PrintString` (`KismetStringLibrary.Conv_IntToString` (`self.Health`)) true true (struct :`R` 1.0 :`G` 0.004101 :`B` 0.134861 :`A` 1.0) 0.0))
    (:`then_1`
      (`KismetSystemLibrary.LineTraceSingle` :`Start` (`self.K2_GetActorLocation`) :`End` (`self.LineTraceFunction`) :`TraceChannel` "TraceTypeQuery1" :`bTraceComplex` true :`DrawDebugType` "ForOneFrame" :`bIgnoreSelf` false :`TraceHitColor` (struct :`R` 0.954931 :`G` 1.0 :`B` 0.986907 :`A` 1.0)))))

(event `mainTime`
  (bind _result (`/Engine/EditorBlueprintResources/StandardMacros.IncrementInt` (`self.Health`))
    (:`  `
      (set `self.Health` _result)
      (`KismetSystemLibrary.PrintString` (`KismetStringLibrary.Conv_IntToString` (`self.LimitHealthFunction`))))))

(fn `LaneTraceFunction_BP`
  (returns (ReturnValue :type "Vector Structure"))
  (return (+ (`self.K2_GetActorLocation`) (* (`KismetMathLibrary.GetForwardVector` (`self.K2_GetActorRotation`)) (`self.MaxDistance`)))))

(fn `UserConstructionScript`)